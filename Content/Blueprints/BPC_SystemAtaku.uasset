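; BPC_SystemAtaku is a component that runs a four-step melee combo (AtakMieczem, "sword attack") on BP_ThirdPersonCharacter's mesh.
; IA_Attack starts an attack when MozeAtakowac allows it, or buffers the press in ZapiszAtak during one.
; IndeksAtakow selects the next DoOnce-guarded, briefly delayed montage, with a kick third.
; AtakMieczemCombo, not called within this graph, continues a buffered combo or resets it through StopCombo.
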(event Custom|AtakMieczem
  ;[0.125 0.125 0.125] Atak Mieczem
  (if (Variables|Default|GetczyAtakuje)
    (Variables|Default|SetzapiszAtak true)
    (else
      (Variables|Default|SetczyAtakuje true)
      (switch int (Variables|Default|GetindeksAtakow)
        (:0
          (CallFunction|Atak1))
        (:1
          (CallFunction|Atak2))
        (:2
          (CallFunction|Atak3))
        (:3
          (CallFunction|Atak4))))))

(event Custom|AtakMieczemCombo
  ;[0.125 0.125 0.125] Kontynuacja combo
  (if (Variables|Default|GetzapiszAtak)
    (Variables|Default|SetzapiszAtak false)
    (switch int (Variables|Default|GetindeksAtakow)
      (:0
        (CallFunction|Atak1))
      (:1
        (CallFunction|Atak2))
      (:2
        (CallFunction|Atak3))
      (:3
        (CallFunction|Atak4)))
    (else
      (CallFunction|StopCombo))))

(event Custom|Atak2
  ;[0.125 0.125 0.125] Atak 2
  (Utilities|FlowControl|DoOnce false :!label _label
    (:Completed
      (Utilities|FlowControl|Delay 0.1)
      (Animation|Montage|PlayMontage (Variables|Default|GetpostacMesh) "/Game/Characters/Mannequins/Animations/AtakMieczem/Attack2_Montage.Attack2_Montage"
        (:then
          (Variables|Default|SetindeksAtakow 2)
          (goto _label Reset))))))

(event Custom|StopCombo
  ;[0.125 0.125 0.125] Zatrzymaj atak/combo
  (Variables|Default|SetczyAtakuje false)
  (Variables|Default|SetindeksAtakow 0))

(event Custom|Atak3
  ;[0.125 0.125 0.125] Atak 3
  (Utilities|FlowControl|DoOnce false :!label _label
    (:Completed
      (Utilities|FlowControl|Delay 0.1)
      (Animation|Montage|PlayMontage (Variables|Default|GetpostacMesh) "/Game/Characters/Mannequins/Animations/AtakMieczem/Kick_Montage.Kick_Montage"
        (:then
          (Variables|Default|SetindeksAtakow 3)
          (goto _label Reset))))))

(event Custom|Atak4
  ;[0.125 0.125 0.125] Atak 4
  (Utilities|FlowControl|DoOnce false :!label _label
    (:Completed
      (Utilities|FlowControl|Delay 0.1)
      (Animation|Montage|PlayMontage (Variables|Default|GetpostacMesh) "/Game/Characters/Mannequins/Animations/AtakMieczem/Attack3_Montage.Attack3_Montage"
        (:then
          (Variables|Default|SetindeksAtakow 4)
          (goto _label Reset))))))

(event Custom|Atak1
  ;[0.125 0.125 0.125] Atak 1
  (Utilities|FlowControl|DoOnce false :!label _label
    (:Completed
      (Utilities|FlowControl|Delay 0.1)
      (Animation|Montage|PlayMontage (Variables|Default|GetpostacMesh) "/Game/Characters/Mannequins/Animations/AtakMieczem/Attack1_Montage.Attack1_Montage"
        (:then
          (Variables|Default|SetindeksAtakow 1)
          (goto _label Reset))))))

(event Input|EnhancedActionEvents|EnhancedInputActionIA_Attack
  (params (ActionValue :type Boolean) (ElapsedSeconds :type Float%20%28double-precision%29) (TriggeredSeconds :type Float%20%28double-precision%29) (InputAction :type Input%20Action%20Object%20Reference :default "/Game/ThirdPerson/Input/Actions/IA_Attack.IA_Attack"))
  ;[0.125 0.125 0.125] Klawisz Ataku
  (:Started
    (if (Variables|Default|GetmozeAtakowac)
      (CallFunction|AtakMieczem))))

(event EventBeginPlay
  (bind _asbp_third_person_character (Utilities|Casting|CastToBP_ThirdPersonCharacter (Components|GetOwner)))
  (Variables|Default|SetpostacMesh (Variables|/Script/Engine.Character|GetMesh _asbp_third_person_character)))